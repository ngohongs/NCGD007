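; Player pawn for a sphere that moves by line-trace-checked teleport steps, turns by yaw via Enhanced Input, and opens a level at the finish.
; Overlapping either pickup type increments one shared AbilityIndex, so pickup count rather than type selects the ability.
; The ability input starts a timer that Tick counts down, running Levitate (gravity off, raised height) or Crusher time slow-down on a latched index.
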(event `self.ReceiveBeginPlay`
  (bind _asplayer_controller (cast `PlayerController` (`self.GetController`)))
  (message `EnhancedInputSubsystemInterface.AddMappingContext` (pcsubsystem `EnhancedInputLocalPlayerSubsystem` _asplayer_controller) "/Game/Input/IMC_InputMapping.IMC_InputMapping" 0 (struct)))

(event `EnhancedInput|/Game/Input/IA_Move`
  (params (ActionValue :type "Float (double-precision)") (ElapsedSeconds :type "Float (double-precision)") (TriggeredSeconds :type "Float (double-precision)") (InputAction :type "InputAction Object Reference" :default "/Game/Input/IA_Move.IA_Move"))
  (bind _returnvalue_x (`KismetMathLibrary.BreakVector` (`SceneComponent.K2_GetComponentScale` (`self.Sphere`))))
  (bind _returnvalue (+ (`SceneComponent.K2_GetComponentLocation` (`self.Sphere`)) (* (* ActionValue (`self.BallSpeed`)) (`SceneComponent.GetForwardVector` (`self.Sphere`)))))
  (:`Triggered`
    (bind _outhit (`KismetSystemLibrary.LineTraceSingleByProfile` (`SceneComponent.K2_GetComponentLocation` (`self.Sphere`)) (+ _returnvalue (+ (* (* ActionValue (`SceneComponent.GetForwardVector` (`self.Sphere`))) (* _returnvalue_x 50.0)) (0.0 0.0 -20.0)))))
    (if (`GameplayStatics.BreakHitResult` _outhit)
      (`KismetSystemLibrary.PrintString` "No Movement")
      (else
        (`self.K2_SetActorLocation` _returnvalue)))))

(event `EnhancedInput|/Game/Input/IA_Turn`
  (params (ActionValue :type "Float (double-precision)") (ElapsedSeconds :type "Float (double-precision)") (TriggeredSeconds :type "Float (double-precision)") (InputAction :type "InputAction Object Reference" :default "/Game/Input/IA_Turn.IA_Turn"))
  (:`Triggered`
    (`SceneComponent.K2_AddRelativeRotation` (`self.Sphere`) (`KismetMathLibrary.MakeRotator` 0.0 0.0 (* ActionValue (`self.TurnDegrees`))) false false)))

(event `EnhancedInput|/Game/Input/IA_Ability`
  (params (ActionValue :type Boolean) (ElapsedSeconds :type "Float (double-precision)") (TriggeredSeconds :type "Float (double-precision)") (InputAction :type "InputAction Object Reference" :default "/Game/Input/IA_Ability.IA_Ability"))
  (bind (_returnvalue_x _returnvalue_y _returnvalue_z) (`KismetMathLibrary.BreakVector` (`SceneComponent.K2_GetComponentLocation` (`self.Sphere`))))
  (:`Triggered`
    (if (and (<= (`self.AbilityDuration`) 0.0) (> (`self.AbilityIndex`) 0))
      (set `self.GroundHeight` _returnvalue_z)
      (bind _output_get (set `self.AbilityDuration` 3.0))
      (`KismetSystemLibrary.PrintString` (`KismetStringLibrary.Conv_DoubleToString` _output_get)))))

(event `self.Sphere.OnComponentHit`
  (params (HitComponent :type "PrimitiveComponent Object Reference") (OtherActor :type "Actor Object Reference") (OtherComp :type "PrimitiveComponent Object Reference") (NormalImpulse :type "Vector Structure") (Hit :type "HitResult Structure (by ref)"))
  (`KismetSystemLibrary.PrintString` (`KismetSystemLibrary.GetObjectName` OtherActor)))

(event `self.Sphere.OnComponentBeginOverlap`
  (params (OverlappedComponent :type "PrimitiveComponent Object Reference") (OtherActor :type "Actor Object Reference") (OtherComp :type "PrimitiveComponent Object Reference") (OtherBodyIndex :type Integer) (bFromSweep :type Boolean) (SweepResult :type "HitResult Structure (by ref)"))
  (cast `/Game/BP_LevitationBall` OtherActor
    (:`then`
      (`KismetSystemLibrary.PrintString` "Orange")
      (bind _result (`/Engine/EditorBlueprintResources/StandardMacros.IncrementInt` (`self.AbilityIndex`))
        (:`  `
          (`KismetSystemLibrary.PrintString` (`KismetStringLibrary.Conv_IntToString` _result))
          (`self.K2_DestroyActor` OtherActor))))
    (:`CastFailed`
      (cast `/Game/BP_TimeSlowDown` OtherActor
        (:`then`
          (`KismetSystemLibrary.PrintString` "Blue")
          (bind _result_2 (`/Engine/EditorBlueprintResources/StandardMacros.IncrementInt` (`self.AbilityIndex`))
            (:`  `
              (`KismetSystemLibrary.PrintString` (`KismetStringLibrary.Conv_IntToString` _result_2))
              (`self.K2_DestroyActor` OtherActor))))
        (:`CastFailed`
          (cast `/Game/BP_FinishPosition` OtherActor)
          (`KismetSystemLibrary.PrintString` "Finish")
          (`GameplayStatics.OpenLevelBySoftObjectPtr` "/Game/World.World"))))))

(event `self.ReceiveTick`
  (params (DeltaSeconds :type "Float (single-precision)"))
  (bind _crusher (`self.Crusher`))
  (bind _abilityduration (`self.AbilityDuration`))
  (if (> (`self.AbilityDuration`) 0.0)
    (bind _output_get (set `self.AbilityDuration` (`KismetMathLibrary.FMax` (- (`self.AbilityDuration`) DeltaSeconds) 0.0)))
    (`KismetSystemLibrary.PrintString` (`KismetStringLibrary.Conv_DoubleToString` _output_get))
    (switch `int` (`self.ExecutedAbilityIndex`)
      (:`0`
        _)
      (:`1`
        (`PrimitiveComponent.SetEnableGravity` (`self.Sphere`) false)
        (`self.K2_SetActorLocation` (`KismetMathLibrary.MakeVector` (.x (`SceneComponent.K2_GetComponentLocation` (`self.Sphere`))) (.y (`SceneComponent.K2_GetComponentLocation` (`self.Sphere`))) (+ (`self.GroundHeight`) 100.0)))
        (if (<= _abilityduration 0.0)
          (`KismetSystemLibrary.PrintString` "Enable Gravity")
          (`PrimitiveComponent.SetEnableGravity` (`self.Sphere`) true)))
      (:`2`
        (`/Game/BP_Crusher.Time Slow Down` _crusher)
        (if (<= _abilityduration 0.0)
          (`/Game/BP_Crusher.Time Speed Up` _crusher))))
    (if (<= _abilityduration 0.0)
      (set `self.ExecutedAbilityIndex` (`self.AbilityIndex`)))
    (else
      (set `self.ExecutedAbilityIndex` (`self.AbilityIndex`)))))

(fn `IsFloorBlock`
  (params (Object :type "Object Object Reference"))
  (returns (`Is Floor` :type Boolean))
  (cast `/Game/BP_Floor` Object
    (:`then`
      _)
    (:`CastFailed`
      (cast `/Game/BP_Step` Object
        (:`then`
          _)
        (:`CastFailed`
          (return false)))))
  (return true))

(fn `UserConstructionScript`)