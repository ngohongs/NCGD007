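; BP_Crusher is a moving hazard that sends the player back to its starting position on contact.
; A Timeline played at Speed drives the actor's Z offset between its start height and MaxHeight.
; A Cube hit by BP_PlayerPawn resets the Player reference to the Sphere location and rotation cached at BeginPlay.
; TimeSlowDown and TimeSpeedUp switch the Timeline between quarter and normal rate for a slow-time effect.
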(event `self.ReceiveBeginPlay`
  (bind _sphere (`/Game/BP_PlayerPawn.Sphere` (`self.Player`)))
  (set `self.InitialPlayerLocation` (`SceneComponent.K2_GetComponentLocation` _sphere))
  (set `self.InitialPlayerRotation` (`SceneComponent.K2_GetComponentRotation` _sphere))
  (bind _output_get (set `self.InitialLocation` (`self.K2_GetActorLocation`)))
  (`TimelineComponent.SetPlayRate` (`self.Timeline`) (`self.Speed`))
  (bind (_direction _track_0) (`Timeline|Timeline`)
    (:`Update`
      (`self.K2_SetActorLocation` (`KismetMathLibrary.MakeVector` (.x _output_get) (.y _output_get) (+ (.z _output_get) (`KismetMathLibrary.Lerp` 0.0 (`self.MaxHeight`) _track_0)))))))

(event `self.Cube.OnComponentHit`
  (params (HitComponent :type "PrimitiveComponent Object Reference") (OtherActor :type "Actor Object Reference") (OtherComp :type "PrimitiveComponent Object Reference") (NormalImpulse :type "Vector Structure") (Hit :type "HitResult Structure (by ref)"))
  (`KismetSystemLibrary.PrintString` "Crush")
  (cast `/Game/BP_PlayerPawn` OtherActor)
  (`self.K2_SetActorLocationAndRotation` (`self.Player`) (`self.InitialPlayerLocation`) (`self.InitialPlayerRotation`) false false))

(event `Time Slow Down`
  (`TimelineComponent.SetPlayRate` (`self.Timeline`) (* (`self.Speed`) 0.25)))

(event `Time Speed Up`
  (`TimelineComponent.SetPlayRate` (`self.Timeline`) (`self.Speed`)))

(fn `UserConstructionScript`)